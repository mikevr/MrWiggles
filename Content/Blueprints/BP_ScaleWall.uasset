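; BP_ScaleWall is a wall whose three cube pieces stretch along Y as the player tilts the headset sideways.
; Each Tick maps HMD roll in either direction to a clamped factor, multiplied by a separate scale amount for the middle, R1 and R2 cubes.
; The scaling runs only while RoomControl is true, which Tick sets after a delay once the first BP_MrWiggles found at BeginPlay has HMDControl enabled.
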(event EventBeginPlay
  (bind _outactors (Actor|GetAllActorsOfClass "/Game/Blueprints/BP_MrWiggles.BP_MrWiggles_C")))

(event EventActorBeginOverlap
  (params (OtherActor :type Actor%20Object%20Reference)))

(event EventTick
  (params (DeltaSeconds :type Float%20%28single-precision%29))
  (bind _devicerotation (Class|HeadMountedDisplayFunctionLibrary|GetOrientationandPosition))
  (bind _maincubescale (Variables|Default|GetmainCubeScale))
  (bind _r1cubescale (Variables|Default|Getr1CubeScale))
  (bind _r2cubescale (Variables|Default|Getr2CubeScale))
  (bind _returnvalue (Math|Float|MapRangeClamped (.roll _devicerotation) 0.0 3e+01 0.0 1.0))
  (bind _returnvalue_2 (Math|Float|MapRangeClamped (.roll _devicerotation) 0.0 -3e+01 0.0 1.0))
  (Utilities|FlowControl|Sequence
    (:then_0
      (if (Variables|Default|GetRoomControl)
        (Utilities|FlowControl|Sequence
          (:then_0
            ;[1 1 1] ScalingTheWall in + Roll
            (Transformation|SetRelativeScale3D (Variables|Default|GetCube_Middle) (Math|Vector|MakeVector 1.0 (+ (* _maincubescale _returnvalue) 1.0 (* _maincubescale _returnvalue_2)) 1.0)))
          (:then_1
            (Transformation|SetRelativeScale3D (Variables|Default|GetCube_R1_01) (Math|Vector|MakeVector 1.0 (+ (* _r1cubescale _returnvalue) 1.0 (* _r1cubescale _returnvalue_2)) 1.0)))
          (:then_2
            (Transformation|SetRelativeScale3D (Variables|Default|GetCube_R2_01) (Math|Vector|MakeVector 1.0 (+ (* _r2cubescale _returnvalue) 1.0 (* _r2cubescale _returnvalue_2)) 1.0))))))
    (:then_1
      (if (Variables|/Game/Blueprints/BP_MrWiggles.BP_MrWiggles_C|GetHMDControl (Utilities|Array|Get(acopy) (stale EventBeginPlay _outactors)))
        (Utilities|FlowControl|Delay 1e+01)
        (Variables|Default|SetRoomControl true)))))

(fn ConstructionScript)