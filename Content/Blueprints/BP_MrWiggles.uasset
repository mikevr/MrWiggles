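; BP_MrWiggles is an actor whose mesh rotates and scales in response to the VR pawn's camera when HMDControl is on.
; BeginPlay picks a random rotation offset, zeroes the scale offset, and only afterwards records the mesh's starting transform.
; Tick adds scaled camera yaw to all rotation axes and divided camera roll to scale, printing debug values.
; The looping one-second timer fires an empty event.
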(event Custom|CustomTimer)

(event EventBeginPlay
  (bind _mrwigglesmesh (Variables|Default|GetMrWigglesMesh))
  (bind _maxrotation (Variables|Default|GetMaxRotation))
  (bind _returnvalue (Transformation|GetWorldRotation _mrwigglesmesh))
  (Utilities|FlowControl|Sequence
    (:then_0
      (Utilities|Time|SetTimerbyEvent (delegate Custom|CustomTimer) 1.0 true)
      (Variables|Default|SetrandomScale (Math|Vector|MakeVector 0.0 0.0 0.0))
      (Variables|Default|SetrandomRotation (Math|Vector|MakeVector (Math|Random|RandomFloatinRange (.x (Variables|Default|GetstartRotation)) _maxrotation) (Math|Random|RandomFloatinRange (.y (Variables|Default|GetstartRotation)) _maxrotation) (Math|Random|RandomFloatinRange (.z (Variables|Default|GetstartRotation)) _maxrotation))))
    (:then_1
      (Variables|Default|SetstartScale (Transformation|GetWorldScale (Variables|Default|GetMrWigglesMesh)))
      (Variables|Default|SetstartRotation (Math|Vector|MakeVector (.roll _returnvalue) (.pitch _returnvalue) (.yaw _returnvalue))))))

(event EventTick
  (params (DeltaSeconds :type Float%20%28single-precision%29))
  (bind _randomrotation (Variables|Default|GetrandomRotation))
  (Development|PrintString (Utilities|String|ToString(Float) (Math|Float|MapRangeClamped (.x (.DevicePosition (Class|HeadMountedDisplayFunctionLibrary|GetOrientationandPosition))) -1e+02 1e+02 0.1 1.0)))
  (if (Variables|Default|GetHMDControl)
    (bind _outactors (Actor|GetAllActorsOfClass "/Game/Blueprints/VRPawn.VRPawn_C"))
    (Utilities|FlowControl|Sequence
      (:then_0
        ;[1 1 1] Yaw To Rotation
        (Transformation|SetWorldRotation (Variables|Default|GetMrWigglesMesh) (Math|Rotator|MakeRotator (.x (+ (Math|Vector|MakeVector (.x _randomrotation) (.y _randomrotation) (.z _randomrotation)) (* (.yaw (Transformation|GetWorldRotation (Variables|/Game/Blueprints/VRPawn.VRPawn_C|GetCamera (Utilities|Array|Get(acopy) _outactors)))) (Variables|Default|GetrotationSpeed)))) (.y (+ (Math|Vector|MakeVector (.x _randomrotation) (.y _randomrotation) (.z _randomrotation)) (* (.yaw (Transformation|GetWorldRotation (Variables|/Game/Blueprints/VRPawn.VRPawn_C|GetCamera (Utilities|Array|Get(acopy) _outactors)))) (Variables|Default|GetrotationSpeed)))) (.z (+ (Math|Vector|MakeVector (.x _randomrotation) (.y _randomrotation) (.z _randomrotation)) (* (.yaw (Transformation|GetWorldRotation (Variables|/Game/Blueprints/VRPawn.VRPawn_C|GetCamera (Utilities|Array|Get(acopy) _outactors)))) (Variables|Default|GetrotationSpeed))))) false false))
      (:then_1
        (Transformation|SetWorldScale3D (Variables|Default|GetMrWigglesMesh) (+ (Variables|Default|GetrandomScale) (/ (.roll (Transformation|GetWorldRotation (Variables|/Game/Blueprints/VRPawn.VRPawn_C|GetCamera (Utilities|Array|Get(acopy) _outactors)))) (Variables|Default|GetscaleSpeed))))
        (Development|PrintString (Utilities|String|ToString(Float) (.roll (Transformation|GetWorldRotation (Variables|/Game/Blueprints/VRPawn.VRPawn_C|GetCamera (Utilities|Array|Get(acopy) _outactors))))))))))

(fn ConstructionScript)