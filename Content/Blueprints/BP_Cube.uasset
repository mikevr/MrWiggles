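; BP_Cube is a cube actor whose material glow reacts to the VR player.
; When a VRPawn's CollisionPlayer overlaps the Cube, a timeline animates the GlowScale parameter and holds an Overlap flag until finished.
; The GlowFlow event plays a randomly flickering glow unless that flag is set.
; Its looping timer and a zero-gravity physics float driven by WigglesGameMode are both disconnected and never run.
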(event Custom|GlowFlow
  (if (not (Variables|Default|GetOverlap))
    (bind _glowstrength (Timeline|Glower Play)
      (:Update
        (Rendering|Material|SetScalarParameterValueonMaterials (Variables|Default|GetCube) "GlowScale" (+ _glowstrength (Math|Random|RandomFloatinRange 0.0 0.2)))))))

(event EventTick
  (params (DeltaSeconds :type Float%20%28single-precision%29)))

(event EventBeginPlay)

(event Collision|EventActorBeginOverlap
  (params (OtherActor :type Actor%20Object%20Reference))
  (bind _asvrpawn (Utilities|Casting|CastToVRPawn OtherActor))
  (if (Class|PrimitiveComponent|IsOverlappingComponent (Variables|/Game/Blueprints/VRPawn.VRPawn_C|GetCollisionPlayer _asvrpawn) (Variables|Default|GetCube))
    (Variables|Default|SetOverlap true)
    (bind _glowstrength (Timeline|GlowStrenth Play)
      (:Update
        (Rendering|Material|SetScalarParameterValueonMaterials (Variables|Default|GetCube) "GlowScale" _glowstrength))
      (:Finished
        (Variables|Default|SetOverlap false)))))

(fn ConstructionScript)