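; BP_VRController is a VR gaze-teleport controller that lets the player jump to the point the camera looks at.
; Each tick it stores the headset yaw, traces from the camera and moves LookAtSphere to the hit at a fixed height.
; Space moves the player capsule to that hit, keeping its height, then sets camera rotation from headset pitch and roll, with a yaw expression that reduces to the stored yaw.
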(event EventTick
  (params (DeltaSeconds :type Float%20%28single-precision%29))
  (bind _camera (Variables|Default|GetCamera))
  (bind _returnvalue (Transformation|GetWorldLocation _camera))
  (Utilities|FlowControl|Sequence
    (:then_0
      ;[1 1 1] Pak deze voor teleport
      (bind _output_get (Variables|Default|SetYawOLD (.yaw (.DeviceRotation (Class|HeadMountedDisplayFunctionLibrary|GetOrientationandPosition))))))
    (:then_1
      (bind _outhit (Collision|LineTraceByChannel _returnvalue (+ _returnvalue (* (Math|Vector|GetForwardVector (Transformation|GetWorldRotation _camera)) (Variables|Default|GetLookAtDistance))) "TraceTypeQuery1" false 0 "None"))
      (Transformation|SetWorldLocation (Variables|Default|GetLookAtSphere) (Math|Vector|MakeVector (.X (Math|Vector|BreakVector (.Location (Collision|BreakHitResult _outhit)))) (.Y (Math|Vector|BreakVector (.Location (Collision|BreakHitResult _outhit)))) 1e+01) false true)
      (Development|PrintString "Hello"))))

(event Input|KeyboardEvents|SpaceBar
  (params (Key :type Key%20Structure :default "AnyKey"))
  (bind _devicerotation (Class|HeadMountedDisplayFunctionLibrary|GetOrientationandPosition))
  (:Pressed
    (Transformation|SetWorldLocation (Variables|/Script/Engine.Character|GetCapsuleComponent (Game|GetPlayerCharacter 0)) (Math|Vector|MakeVector (.X (Math|Vector|BreakVector (.Location (Collision|BreakHitResult (stale EventTick _outhit))))) (.Y (Math|Vector|BreakVector (.Location (Collision|BreakHitResult (stale EventTick _outhit))))) (.Z (Math|Vector|BreakVector (Transformation|GetWorldLocation (Variables|/Script/Engine.Character|GetCapsuleComponent (Game|GetPlayerCharacter 0)))))) false true)
    ;[1 1 1] Pak deze na teleport
    (bind _output_get (Variables|Default|SetYawNew (.yaw _devicerotation)))
    (Transformation|SetWorldRotation (Variables|Default|GetCamera) (Math|Rotator|MakeRotator (.roll _devicerotation) (.pitch _devicerotation) (* (/ (stale EventTick _output_get) _output_get) (Variables|Default|GetYawNew))) false false)))

(fn ConstructionScript)