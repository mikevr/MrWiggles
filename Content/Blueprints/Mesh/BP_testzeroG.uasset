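; BP_testzeroG is a test actor whose static mesh floats when zero gravity is active in the game mode.
; Each Tick it reads ZeroG from WigglesGameMode and, when true, disables mesh gravity, enables physics and plays the Gravity timeline.
; The timeline's GravityForce, randomly scaled on each update, pushes the mesh along Z, and nothing restores gravity afterward.
; A VRPawn whose CollisionPlayer overlaps the mesh triggers a debug "Hello" print.
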(event EventBeginPlay)

(event EventTick
  (params (DeltaSeconds :type Float%20%28single-precision%29))
  (bind _aswiggles_game_mode (Utilities|Casting|CastToWigglesGameMode (Game|GetGameMode)))
  (if (Variables|/Game/Blueprints/WigglesGameMode.WigglesGameMode_C|GetZeroG _aswiggles_game_mode)
    (Physics|SetEnableGravity (Variables|Default|GetStaticMesh) false)
    (Physics|SetSimulatePhysics (Variables|Default|GetStaticMesh) true)
    (bind _gravityforce (Timeline|Gravity Play)
      (:Update
        (Physics|AddForce (Variables|Default|GetStaticMesh) (Math|Vector|MakeVector 0.0 0.0 (* _gravityforce (Math|Random|RandomFloatinRange 0.1 3.0))) "None" false)))))

(event Collision|EventActorBeginOverlap
  (params (OtherActor :type Actor%20Object%20Reference))
  (bind _asvrpawn (Utilities|Casting|CastToVRPawn OtherActor))
  (if (Class|PrimitiveComponent|IsOverlappingComponent (Variables|/Game/Blueprints/VRPawn.VRPawn_C|GetCollisionPlayer _asvrpawn) (Variables|Default|GetStaticMesh))
    (Development|PrintText "Hello")))

(fn ConstructionScript)