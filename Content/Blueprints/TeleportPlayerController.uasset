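; A player controller that teleports the VR pawn where the camera points when TeleportInput is pressed.
; A camera-forward visibility trace allows the move if the hit actor implements InteractionInterfaceBP.
; The move adds the trace end's X and Y to the capsule as a world offset, rather than setting the hit location.
; TeleporToLocation, uncalled here, instead accepts near-flat surfaces by normal and only draws a debug cylinder.
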(event EventBeginPlay
  (bind _asvrpawn (Utilities|Casting|CastToVRPawn (Game|GetPlayerCharacter 0)))
  (Variables|Default|SetVRPAwn _asvrpawn))

(event Input|ActionEvents|InputActionTeleportInput
  (params (Key :type Key%20Structure :default "AnyKey"))
  (bind _returnvalue (Game|GetPlayerCameraManager 0))
  (bind _returnvalue_2 (Transformation|GetActorLocation _returnvalue))
  (:Pressed
    (bind _outhit (Collision|LineTraceByChannel _returnvalue_2 (+ _returnvalue_2 (* (Transformation|GetActorForwardVector _returnvalue) (Variables|Default|GetTeleportDistance))) "TraceTypeQuery1" false 0 "ForDuration"))
    (bind _output_get (Variables|Default|SetCanTeleport (Utilities|DoesObjectImplementInterface (.HitActor (Collision|BreakHitResult _outhit)) "/Game/Blueprints/InteractionInterface-BP.InteractionInterface-BP_C")))
    (if _output_get
      (bind _output_get_2 (Variables|Default|SetTeleportLocation (.TraceEnd (Collision|BreakHitResult _outhit))))
      (Transformation|AddWorldOffset (Variables|/Script/Engine.Character|GetCapsuleComponent (Variables|Default|GetVRPAwn)) (Math|Vector|MakeVector (.x _output_get_2) (.y _output_get_2) 0.0) (.bBlockingHit (Collision|BreakHitResult _outhit)) true))))

(fn ConstructionScript)

(fn TeleportoLocation
  (params (Postion :type Vector) (FowardVector :type Vector))
  (bind _outhit (Collision|LineTraceByChannel Postion (+ Postion (* FowardVector 1e+04)) "TraceTypeQuery1" false 0 "ForDuration"))
  (bind _output_get (Variables|Default|SetCanTeleport (> (Math|Vector|DotProduct (.Normal (Collision|BreakHitResult _outhit)) "0, 0,1.000000") 0.9)))
  (if _output_get
    (bind _output_get_2 (Variables|Default|SetTeleportLocation (.Location (Collision|BreakHitResult _outhit))))
    (Class|KismetSystemLibrary|DrawDebugCylinder _output_get_2 (* _output_get_2 (* (.Normal (Collision|BreakHitResult _outhit)) 2e+01)) 5e+01 12 "(R=1.000000,G=1.000000,B=1.000000,A=1.000000)" 0.0)))